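; AutoClick actor, apparently a "grandma" auto-clicker, that places itself randomly and animates a sprite on spawn.
; BeginPlay moves it to a random point in a fixed X/Z rectangle, then a one-shot timeline rotates MotorSprite's yaw.
; When that finishes, the Keyboard sound starts and the LoopGrandma timeline drives the sprite's pitch.
; No click logic lives here, and the debug drawing of the spawn area is unconnected.
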(event EventBeginPlay
  (Utilities|FlowControl|Sequence
    (:then_0
      (bind _output_get (Variables|Default|SetstartPos "0.000000,0.000000,-250.000000"))
      (bind _output_get_2 (Variables|Default|SetmaxPos "500.000000,0.000000,250.000000")))
    (:then_1
      (Variables|Default|SetspawnHeight (.Z (Math|Vector|BreakVector (- (Variables|Default|GetmaxPos) (Variables|Default|GetstartPos)))))
      (Variables|Default|SetspawnWidth (.X (Math|Vector|BreakVector (- (Variables|Default|GetmaxPos) (Variables|Default|GetstartPos))))))
    (:then_2
      (Transformation|SetActorLocation (+ (Math|Vector|MakeVector (* (Variables|Default|GetspawnWidth) (Math|Random|RandomFloat)) 0.0 (* (Variables|Default|GetspawnHeight) (Math|Random|RandomFloat))) (Variables|Default|GetstartPos)) false false)
      (bind _rotation (Timeline|GrandmaTimeline PlayFromStart)
        (:Update
          (Transformation|SetRelativeRotation (Variables|Default|Getmotor_Sprite) (Math|Rotator|MakeRotator 0.0 0.0 _rotation) false false))
        (:Finished
          (Audio|Components|Audio|Play (Variables|Default|GetKeyboard) 0.0)
          (bind _constantrotation (Timeline|LoopGrandma Play)
            (:Update
              (Transformation|SetRelativeRotation (Variables|Default|Getmotor_Sprite) (Math|Rotator|MakeRotator 0.0 _constantrotation 0.0) false false))))))))

(fn ConstructionScript)