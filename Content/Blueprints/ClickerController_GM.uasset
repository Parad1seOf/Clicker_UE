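; Game mode for a clicker game that creates the game UI and tracks the click count up to a maximum.
; AddClick raises the count, refreshes the UI, plays sounds and spawns one AutoClick actor per reached click threshold, carrying the remainder over.
; The first spawn starts a looping timer that adds clicks equal to the spawned actor count, so auto-clicks feed further spawns.
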(event Custom|ActivateTimer
  (Utilities|Time|SetTimerbyEvent (delegate Custom|AddClickEvent) (Variables|Default|GetTimeToClick) true))

(event Custom|AddClickEvent
  (CallFunction|AddClick (Variables|Default|GetActorCounter) "/Game/Sound/Click2.Click2")
  (if (not (Variables|Default|GetMaxValueReached))
    (Default|CallOnUpdateAddedClicksUI)))

(event EventBeginPlay
  (bind _returnvalue (UserInterface|CreateWidget "/Game/UI/GameUI_UW.GameUI_UW_C"))
  (UserInterface|Viewport|AddtoViewport _returnvalue 0))

(fn ConstructionScript)

(fn AddClick
  (params (AddValue :type Integer) (ClickSound :type Sound%20Wave%20Object%20Reference))
  (Variables|Default|SetCounterClicksToNewActor (+ (Variables|Default|GetCounterClicksToNewActor) AddValue))
  (if (> (+ AddValue (Variables|Default|GetClickCount)) (Variables|Default|GetMaxClicks))
    (Variables|Default|SetMaxValueReached true)
    (Variables|Default|SetClickCount (Variables|Default|GetMaxClicks))
    (Default|CallOnUpdateUI)
    (else
      (Variables|Default|SetClickCount (+ AddValue (Variables|Default|GetClickCount)))
      (Default|CallOnUpdateUI)
      (Audio|PlaySound2D ClickSound 0.5 1.0 0.0 0 0)
      (if (>= (Variables|Default|GetCounterClicksToNewActor) (Variables|Default|GetClicksToNewActor))
        (for _index (range 0 (- (.ReturnValue (Math|Float|Division(WholeandRemainder) (Math|Conversions|ToFloat(Integer) (Variables|Default|GetCounterClicksToNewActor)) (Math|Conversions|ToFloat(Integer) (Variables|Default|GetClicksToNewActor)))) 1))
          (Game|SpawnActorfromClass "/Game/Blueprints/AutoClick.AutoClick_C" (Class|Actor|GetLevelTransform) "Undefined" "MultiplyWithRoot" 0 0)
          (Variables|Default|SetActorCounter (+ (Variables|Default|GetActorCounter) 1)))
        (Variables|Default|SetCounterClicksToNewActor (Math|Float|Truncate (.Remainder (Math|Float|Division(WholeandRemainder) (Math|Conversions|ToFloat(Integer) (Variables|Default|GetCounterClicksToNewActor)) (Math|Conversions|ToFloat(Integer) (Variables|Default|GetClicksToNewActor))))))
        (Audio|PlaySound2D "/Game/Sound/10clicks.10clicks" 0.5 1.0 0.0 0 0)
        (Default|CallOnUpdateUI)
        (if (not (Variables|Default|GetIsTimerAviable))
          (Variables|Default|SetIsTimerAviable true)
          (CallFunction|ActivateTimer))))))